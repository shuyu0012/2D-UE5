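; BP_Enemy is a 2D sprite enemy with three data-asset-driven types that chases the player and damages them on overlap.
; A looping timer teleports it to a navmesh point outside player range before starting AI movement.
; Hits trigger knockback, red flash and damage numbers; death parks it below the map, requesting pooled drops and more enemies from the object manager.
; The squirting type periodically fires pooled snow projectiles aimed at the cursor's hit location.
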(event `击退`
  (params (`冲击力` :type "Float (double-precision)"))
  ;[1 1 1] 击退
  (`MovementComponent.StopMovementImmediately` (`self.CharacterMovement`))
  (`self.LaunchCharacter` (* (/ `冲击力` (`self.质量`)) (`KismetMathLibrary.GetDirectionUnitVector` (`self.K2_GetActorLocation` (`GameplayStatics.GetPlayerPawn` 0)) (`self.K2_GetActorLocation`))) true))

(event `开始移动`
  (bind _returnvalue (`GameplayStatics.GetPlayerPawn` 0))
  ;[1 1 1] 移动
  (`KismetSystemLibrary.Delay` 0.2)
  (`/Engine/EditorBlueprintResources/StandardMacros.IsValid` _returnvalue
    (:`Is Valid`
      (`CharacterMovementComponent.SetMovementMode` (`self.CharacterMovement`) "MOVE_Walking" 0)
      (`|AIMoveTo` self (0.0 0.0 0.0) _returnvalue
        (:`OnSuccess`
          (`KismetSystemLibrary.K2_ClearAndInvalidateTimerHandle` (`self.寻路定时器`))
          (`self.开始移动`))
        (:`OnFail`
          (bind _returnvalue_2 (`KismetSystemLibrary.K2_SetTimerDelegate` (`|CreateDelegate` :!event `开始移动`) 0.5 true))
          (set `self.寻路定时器` _returnvalue_2))))))

(event `self.ReceiveBeginPlay`
  ;[1 1 1] 初始化
  (bind _asabp_enemy (cast `/Game/enemy/ABP_Enemy` (`self.GetAnimInstance`)))
  (bind _output_get (set `self.As ABP Enemy` _asabp_enemy))
  (switch `/Game/blueprint/enumerate/EnemyClassification` (`self.敌人分类`)
    (:`NewEnumerator0`
      (set `self.敌人数据资产` "/Game/Data_assets/Enemy_data/DA_Fire_Skull.DA_Fire_Skull"))
    (:`NewEnumerator1`
      (set `self.敌人数据资产` "/Game/Data_assets/Enemy_data/DA_Cyclops.DA_Cyclops"))
    (:`NewEnumerator2`
      (set `self.敌人数据资产` "/Game/Data_assets/Enemy_data/DA_Squirting_monsters.DA_Squirting_monsters")))
  (bind (_id `_名字` `_敌人移动动画` _hp `_敌人攻击` `_敌人移动速度` `_经验值` `_生命周期` `_是否精英` `_质量` `_敌人弹射动画`) (`/Game/Data_assets/Enemy_data/EnemyData.获取敌人信息` (`self.敌人数据资产`)))
  (set `/Game/enemy/ABP_Enemy.敌人移动动画` `_敌人移动动画` _output_get)
  (set `CharacterMovementComponent.MaxWalkSpeed` `_敌人移动速度` (`self.CharacterMovement`))
  (set `self.质量` `_质量`)
  (set `self.HP` _hp)
  (set `self.经验值` `_经验值`)
  (set `self.敌人弹射动画` `_敌人弹射动画`)
  (set `self.敌人攻击` `_敌人攻击`)
  (`KismetSystemLibrary.K2_SetTimer` null "产生敌人正确的出生点" 0.3 true)
  (switch `/Game/blueprint/enumerate/EnemyClassification` (`self.敌人分类`)
    (:`NewEnumerator2`
      (`KismetSystemLibrary.K2_SetTimer` null "雪弹" 2.0 true))))

(event `self.ReceiveTick`
  (params (DeltaSeconds :type "Float (single-precision)"))
  (`self.K2_SetActorRotation` (struct)))

(event `/Game/interface/EnemyInterface.受击`
  (params (`受到的伤害` :type "Float (double-precision)") (`冲击力` :type "Float (double-precision)"))
  ;[1 1 1] 敌人受击
  (bind _returnvalue (`self.敌人HP计算` `受到的伤害`))
  (if _returnvalue
    (`self.敌人死亡判断`)
    (else
      (`PaperFlipbookComponent.SetSpriteColor` (`self.Sprite`) (struct :`R` 1.0 :`A` 1.0))
      (`GameplayStatics.PlaySound2D` "/Game/sound/sound_effect/HitSound.HitSound" 1.0 1.0 0.0 null null)
      (`self.受击显示数字` (`KismetTextLibrary.Conv_IntToText` (`KismetMathLibrary.FTrunc` `受到的伤害`)))
      (`self.击退` `冲击力`)
      (`KismetSystemLibrary.Delay` 0.1)
      (`PaperFlipbookComponent.SetSpriteColor` (`self.Sprite`) (struct :`R` 1.0 :`G` 1.0 :`B` 1.0 :`A` 1.0)))))

(event `self.CapsuleComponent.OnComponentBeginOverlap`
  (params (OverlappedComponent :type "PrimitiveComponent Object Reference") (OtherActor :type "Actor Object Reference") (OtherComp :type "PrimitiveComponent Object Reference") (OtherBodyIndex :type Integer) (bFromSweep :type Boolean) (SweepResult :type "HitResult Structure (by ref)"))
  ;[1 1 1] 敌人碰撞命中
  (if (`self.ActorHasTag` OtherActor "Player")
    (message `/Game/interface/PlayerInterface.玩家受击` OtherActor (`self.敌人攻击`) self)))

(fn `UserConstructionScript`)

(fn `产生敌人正确的出生点`
  (locals (`随机出点` :type "Vector Structure" :default (0.0 0.0 0.0)))
  (bind _randomlocation (`NavigationSystemV1.K2_GetRandomLocationInNavigableRadius` (`self.K2_GetActorLocation` (`GameplayStatics.GetPlayerPawn` 0)) 900.0 null null))
  (set `local.随机出点` _randomlocation)
  (if (not (`/Game/blueprint/instance/PublicLibraries.检查是否在玩家范围内` (`local.随机出点`)))
    (bind _returnvalue (`self.K2_TeleportTo` (+ (`local.随机出点`) (0.0 0.0 15.0))))
    (if _returnvalue
      (`KismetSystemLibrary.K2_ClearTimer` null "产生敌人正确的出生点")
      (`self.SetActorTickEnabled` true)
      (`ActorComponent.SetComponentTickEnabled` (`self.AnimationComponent`) true)
      (set `self.是否死亡` false)
      (`PrimitiveComponent.SetCollisionResponseToChannel` (`self.CapsuleComponent`) "ECC_Pawn" "ECR_Block")
      (`|ExecutionSequence`
        (:`then_0`
          (`self.开始移动`))
        (:`then_1`
          (switch `/Game/blueprint/enumerate/EnemyClassification` (`self.敌人分类`)
            (:`NewEnumerator2`
              (`KismetSystemLibrary.K2_SetTimer` null "雪弹" 2.0 true))))))))

(fn `受击显示数字`
  (params (`伤害数字` :type Text))
  (`self.伤害数字容器`
    (:`then`
      _)
    (:`else`
      (bind _returnvalue (`|SpawnActorFromClass` "/Game/UI/BP_DamageNumber.BP_DamageNumber_C" (`KismetMathLibrary.MakeTransform` (`SceneComponent.K2_GetComponentLocation` (`self.Sprite`))) "AlwaysSpawn" "MultiplyWithRoot" null null))
      (bind _output_get (set `self.伤害数字容器` _returnvalue))
      (`self.K2_AttachToComponent` _output_get (`self.Sprite`) "None" "KeepWorld" "KeepWorld" "KeepWorld" true)))
  (`/Game/UI/BP_DamageNumber.显示伤害数字` _output_get `伤害数字`))

(fn `敌人HP计算`
  (params (`受到的伤害` :type "Float (double-precision)"))
  (returns (ReturnValue :type Boolean))
  (bind _output_get (set `self.HP` (`KismetMathLibrary.FClamp` (- (`self.HP`) `受到的伤害`) 0.0 (`self.HP`))))
  (return (== _output_get 0.0)))

(fn `敌人死亡判断`
  (bind _asbp_player (`/Game/blueprint/instance/PublicLibraries.Get玩家`))
  (`|ExecutionSequence`
    (:`then_0`
      (if (`KismetSystemLibrary.K2_TimerExists` null "雪弹")
        (`KismetSystemLibrary.K2_ClearTimer` null "雪弹")
        (`KismetSystemLibrary.PrintString` "Hello")))
    (:`then_1`
      (set `/Game/enemy/ABP_Enemy.敌人是否死亡` true (`self.As ABP Enemy`))
      (`CharacterMovementComponent.SetMovementMode` (`self.CharacterMovement`) "MOVE_None" 0)
      (set `self.是否死亡` true)
      (`PrimitiveComponent.SetCollisionResponseToChannel` (`self.CapsuleComponent`) "ECC_Pawn" "ECR_Ignore")
      (`KismetSystemLibrary.K2_ClearAndInvalidateTimerHandle` (`self.寻路定时器`))
      (`KismetSystemLibrary.K2_SetTimer` null "敌人死亡后" 0.4)
      (`/Engine/EditorBlueprintResources/StandardMacros.IncrementInt` (`/Game/blueprint/BP_player.击杀数` _asbp_player)
        (:`  `
          (`/Game/blueprint/BP_player.更新击杀数` _asbp_player))))))

(fn `敌人死亡后`
  (locals (`敌人死亡时的位置` :type "Vector Structure"))
  (`GameplayStatics.PlaySound2D` "/Game/sound/sound_effect/EnemyDead.EnemyDead" 1.0 1.0 0.0 null null)
  (`self.SetActorTickEnabled` false)
  (`ActorComponent.SetComponentTickEnabled` (`self.AnimationComponent`) false)
  (set `local.敌人死亡时的位置` (`self.K2_GetActorLocation`))
  (`KismetArrayLibrary.Array_RemoveItem` (`/Game/blueprint/bullet/ObjectManagement.活动的敌人` (`/Game/blueprint/instance/GameInstances.对象管理` (`/Game/blueprint/instance/PublicLibraries.Get游戏实例`))) self)
  (if true
    (bind _returnvalue (`self.K2_TeleportTo` (0.0 0.0 -1000.0)))
    (if _returnvalue
      (`/Game/blueprint/bullet/ObjectManagement.设置道具池` (`/Game/blueprint/instance/GameInstances.对象管理` (`/Game/blueprint/instance/PublicLibraries.Get游戏实例`)) (`self.经验值`) (`local.敌人死亡时的位置`))
      (`/Game/blueprint/bullet/ObjectManagement.产生更多敌人` (`/Game/blueprint/instance/GameInstances.对象管理` (`/Game/blueprint/instance/PublicLibraries.Get游戏实例`))))))

(fn `雪弹`
  (bind _returnvalue (`self.K2_GetActorLocation`))
  (bind (_returnvalue_roll _returnvalue_pitch _returnvalue_yaw) (`KismetMathLibrary.BreakRotator` (`KismetMathLibrary.FindLookAtRotation` _returnvalue (`.Location` (`GameplayStatics.BreakHitResult` (`PlayerController.GetHitResultUnderCursorByChannel` (`GameplayStatics.GetPlayerController` 0) "TraceTypeQuery1" true))))))
  (for _ (range 1)
    (`/Game/blueprint/bullet/ObjectManagement.设置子弹池` (`/Game/blueprint/instance/GameInstances.对象管理` (`/Game/blueprint/instance/PublicLibraries.Get游戏实例`)) _returnvalue "/Game/bullet/Snow_bombs/IceSpike_雪弹.IceSpike_雪弹" (`self.敌人攻击`) (* (`KismetMathLibrary.Conv_RotatorToVector` (`KismetMathLibrary.MakeRotator` 0.0 0.0 _returnvalue_yaw)) 100) (1.0 1.0 1.0) (1.0 1.0 1.0) "Player" 2.0 15.0)))