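; BP_Prop is a pooled pickup (coin, heart or octopus) that picks its flipbook from its category on BeginPlay.
; Sphere overlap starts a timeline that interpolates the prop toward the overlapping actor.
; When close, it sends 接收道具 to that actor and recycles itself by switching state, moving off-stage and playing a sound for coins.
; 传递道具池信息 stores an experience value and sets the other pool state.
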(event `self.ReceiveBeginPlay`
  (switch `/Game/blueprint/enumerate/ItemClassification` (`self.道具分类`)
    (:`NewEnumerator1`
      (set `self.道具图形序列` "/Game/道具/金币/道具_金币.道具_金币"))
    (:`NewEnumerator0`
      (set `self.道具图形序列` "/Game/道具/心/道具_心.道具_心"))
    (:`NewEnumerator2`
      (set `self.道具图形序列` "/Game/道具/章鱼/道具_章鱼.道具_章鱼")))
  (`PaperFlipbookComponent.SetFlipbook` (`self.PaperFlipbook`) (`self.道具图形序列`)))

(event `self.Sphere.OnComponentBeginOverlap`
  (params (OverlappedComponent :type "PrimitiveComponent Object Reference") (OtherActor :type "Actor Object Reference") (OtherComp :type "PrimitiveComponent Object Reference") (OtherBodyIndex :type Integer) (bFromSweep :type Boolean) (SweepResult :type "HitResult Structure (by ref)"))
  (set `self.拾取对象` OtherActor)
  (`Timeline|飞向拾取者` :!via `PlayFromStart`
    (:`Update`
      (`self.K2_SetActorLocation` (`KismetMathLibrary.VInterpTo` (`self.K2_GetActorLocation`) (`self.K2_GetActorLocation` (`self.拾取对象`)) (`GameplayStatics.GetWorldDeltaSeconds`) 5.0))
      (if (< (`self.GetDistanceTo` self (`self.拾取对象`)) 5.0)
        (message `/Game/interface/PlayerInterface.接收道具` (`self.拾取对象`) self)
        (`TimelineComponent.Stop` (`self.飞向拾取者`))
        (`self.回收道具池`)))))

(fn `UserConstructionScript`)

(fn `传递道具池信息`
  (params (`经验值` :type Integer))
  (set `self.经验值` `经验值`)
  (set `self.道具对象状态` "NewEnumerator0"))

(fn `回收道具池`
  (set `self.道具对象状态` "NewEnumerator1")
  (`self.K2_SetActorLocation` (200.0 200.0 -1000.0))
  (switch `/Game/blueprint/enumerate/ItemClassification` (`self.道具分类`)
    (:`NewEnumerator1`
      (set `self.拾取道具音效` "/Game/sound/sound_effect/Coins.Coins"))
    (:`NewEnumerator0`
      (set `self.拾取道具音效` null))
    (:`NewEnumerator2`
      (set `self.拾取道具音效` null)))
  (bind `_拾取道具音效` (`self.拾取道具音效`)
    (:`then`
      (`GameplayStatics.PlaySound2D` `_拾取道具音效` 1.0 1.0 0.0 null null))
    (:`else`)))