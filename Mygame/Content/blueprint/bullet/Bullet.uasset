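; Pooled projectile actor that shows a flipbook sprite, moves by ProjectileMovement and damages whatever its Sphere overlaps.
; A setup function applies sprite, damage, velocity, scales, target tag, impact and a lifetime timer.
; The target tag selects an enemy hit message, sent once per actor, or a player hit message.
; When the timer fires, the bullet clears its sprite and hit list, teleports away and flips state rather than being destroyed.
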(event `self.Sphere.OnComponentBeginOverlap`
  (params (OverlappedComponent :type "PrimitiveComponent Object Reference") (OtherActor :type "Actor Object Reference") (OtherComp :type "PrimitiveComponent Object Reference") (OtherBodyIndex :type Integer) (bFromSweep :type Boolean) (SweepResult :type "HitResult Structure (by ref)"))
  (switch `name` (`self.命中对象标签`)
    (:`敌人`
      (if (not (`KismetArrayLibrary.Array_Contains` (`self.命中的对象`) OtherActor))
        (`KismetArrayLibrary.Array_AddUnique` (`self.命中的对象`) OtherActor)
        (message `/Game/interface/EnemyInterface.受击` OtherActor (`self.子弹伤害`) (`self.冲击力`))))
    (:`Player`
      (message `/Game/interface/PlayerInterface.玩家受击` OtherActor (`self.子弹伤害`) self))))

(fn `UserConstructionScript`)

(fn `子弹对象回收`
  (`PaperFlipbookComponent.SetFlipbook` (`self.PaperFlipbook`) null)
  (`self.K2_SetActorLocation` (10000.0 10000.0 -1000.0))
  (set `self.子弹对象状态` "NewEnumerator1")
  (`KismetArrayLibrary.Array_Clear` (`self.命中的对象`)))

(fn `设置子弹属性`
  (params (`子弹图形` :type "PaperFlipbook Object Reference") (`子弹伤害` :type "Float (double-precision)") (`子弹速度` :type "Vector Structure") (`子弹大小` :type "Vector Structure") (`命中范围` :type "Vector Structure") (`命中对象标签` :type Name) (`生命周期` :type "Float (double-precision)") (`冲击力` :type "Float (double-precision)"))
  (`PaperFlipbookComponent.SetFlipbook` (`self.PaperFlipbook`) `子弹图形`)
  (set `self.子弹伤害` `子弹伤害`)
  (set `MovementComponent.Velocity` `子弹速度` (`self.ProjectileMovement`))
  (`SceneComponent.SetWorldScale3D` (`self.PaperFlipbook`) `子弹大小`)
  (`SceneComponent.SetWorldScale3D` (`self.Sphere`) `命中范围`)
  (set `self.命中对象标签` `命中对象标签`)
  (set `self.子弹对象状态` "NewEnumerator0")
  (set `self.冲击力` (`local.冲击力`))
  (`KismetSystemLibrary.K2_SetTimer` null "子弹对象回收" `生命周期`))