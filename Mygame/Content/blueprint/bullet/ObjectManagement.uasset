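; Object manager that pools bullets, enemies and experience props, registering itself on the game instance at BeginPlay.
; Each pool reuses an object in its free state or spawns one out of view below the origin.
; It fills enemies to a target count, randomizing new spawns' types once time and player-level thresholds are met.
; A looping one-second timer tracks level time and updates the player's status UI.
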(event `self.ReceiveBeginPlay`
  (set `/Game/blueprint/instance/GameInstances.对象管理` self (`/Game/blueprint/instance/PublicLibraries.Get游戏实例`))
  (`self.设置产生的敌人数量` (`self.敌人数量`))
  (bind _returnvalue (`KismetSystemLibrary.K2_SetTimerDelegate` (`|CreateDelegate` :!event `关卡计时`) 1.0 true))
  (set `self.关卡计时定时器` _returnvalue))

(event `关卡计时`
  (bind `_计时时间` (`self.计时时间`))
  (`/Engine/EditorBlueprintResources/StandardMacros.IncrementInt` `_计时时间`
    (:`  `
      (`/Game/UI/UI_State.更新时间` (`/Game/blueprint/BP_player.UI状态` (`/Game/blueprint/instance/PublicLibraries.Get玩家`)) (/ `_计时时间` 60) (mod `_计时时间` 60)))))

(fn `UserConstructionScript`)

(fn `产生更多敌人`
  (if (< (`KismetArrayLibrary.Array_Length` (`self.活动的敌人`)) (`self.敌人数量`))
    (`self.设置敌人池`)))

(fn `设置产生的敌人数量`
  (params (`敌人数量` :type Integer))
  (for _ (range `敌人数量`)
    (`self.设置敌人池`)))

(fn `设置子弹池`
  (params (`子弹发射位置` :type "Vector Structure") (`子弹图形` :type "PaperFlipbook Object Reference") (`子弹伤害` :type "Float (double-precision)") (`子弹速度` :type "Vector Structure") (`子弹大小` :type "Vector Structure") (`命中范围` :type "Vector Structure") (`命中对象标签` :type Name) (`生命周期` :type "Float (double-precision)") (`冲击力` :type "Float (double-precision)"))
  (locals (`子弹` :type "/Game/blueprint/bullet/Bullet Object Reference"))
  (bind `_子弹` (`local.子弹`))
  (for _array_element (`self.子弹池`)
    (if (`|EnumEquality` (`/Game/blueprint/bullet/Bullet.子弹对象状态` _array_element) "NewEnumerator1")
      (set `local.子弹` _array_element)
      (break)))
  (`local.子弹`
    (:`then`
      _)
    (:`else`
      (bind _returnvalue (`|SpawnActorFromClass` "/Game/blueprint/bullet/Bullet.Bullet_C" (`KismetMathLibrary.MakeTransform` (10000.0 10000.0 -1000.0)) "Undefined" "MultiplyWithRoot" null null))
      (bind _output_get (set `local.子弹` _returnvalue))
      (`KismetArrayLibrary.Array_Add` (`self.子弹池`) _output_get)))
  (`/Game/blueprint/bullet/Bullet.设置子弹属性` `_子弹` `子弹图形` `子弹伤害` `子弹速度` `子弹大小` `命中范围` `命中对象标签` `生命周期` `冲击力`)
  (`self.K2_SetActorLocation` `_子弹` `子弹发射位置` false false))

(fn `设置敌人池`
  (locals (`敌人` :type "/Game/enemy/BP_Enemy Object Reference"))
  (for _array_element (`self.敌人池`)
    (if (`|EnumEquality` (`/Game/enemy/BP_Enemy.敌人对象状态` _array_element) "NewEnumerator1")
      (set `local.敌人` _array_element)
      (break)))
  (`local.敌人`
    (:`then`
      _)
    (:`else`
      (if (not (and (>= (`self.计时时间`) 30) (>= (`/Game/blueprint/BP_player.等级` (`/Game/blueprint/instance/PublicLibraries.Get玩家`)) 5)))
        (set `self.敌人分类` "NewEnumerator0" :!label _label)
        (else
          (switch `int` (`KismetMathLibrary.RandomIntegerInRange` 0 (`self.敌人种类数`))
            (:`0`
              (goto _label))
            (:`1`
              (set `self.敌人分类` "NewEnumerator1" :!label _label_2))
            (:`2`
              (goto _label_2))
            (:`3`
              (set `self.敌人分类` "NewEnumerator2")))))
      (bind _returnvalue (`|SpawnActorFromClass` "/Game/enemy/BP_Enemy.BP_Enemy_C" (`KismetMathLibrary.MakeTransform` (0.0 0.0 -1000.0)) "Undefined" "MultiplyWithRoot" null (`self.敌人分类`) null))
      (set `local.敌人` _returnvalue)
      (`KismetArrayLibrary.Array_AddUnique` (`self.敌人池`) (`local.敌人`))))
  (set `/Game/enemy/BP_Enemy.敌人对象状态` "NewEnumerator0" (`local.敌人`))
  (`KismetArrayLibrary.Array_Add` (`self.活动的敌人`) (`local.敌人`)))

(fn `设置道具池`
  (params (`经验值` :type Integer) (`位置` :type "Vector Structure"))
  (locals (`道具` :type "/Game/道具/BP_Prop Object Reference"))
  (for _array_element (`self.道具池`)
    (if (`|EnumEquality` (`/Game/道具/BP_Prop.道具对象状态` _array_element) "NewEnumerator1")
      (set `local.道具` _array_element)
      (break)))
  (`local.道具`
    (:`then`
      _)
    (:`else`
      (bind _returnvalue (`|SpawnActorFromClass` "/Game/道具/BP_Prop.BP_Prop_C" (`KismetMathLibrary.MakeTransform` (200.0 200.0 -1000.0)) "Undefined" "MultiplyWithRoot" null null))
      (bind _output_get (set `local.道具` _returnvalue))
      (`KismetArrayLibrary.Array_AddUnique` (`self.道具池`) _output_get)))
  (`/Game/道具/BP_Prop.传递道具池信息` (`local.道具`) (`local.经验值`))
  (`self.K2_SetActorLocation` (`local.道具`) (`local.位置`) false false))