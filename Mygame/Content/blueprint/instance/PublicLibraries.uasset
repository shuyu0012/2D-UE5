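; Blueprint library of shared helper functions for reaching common game objects and testing on-screen visibility.
; Two getters return the game instance cast to GameInstances and player 0's pawn cast to BP_player.
; The range check (检查是否在玩家范围内) projects a world location through player 0's controller and tests whether it lands inside the viewport bounds, rather than measuring distance.
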(fn `Get游戏实例`
  (returns (`As游戏实例` :type "/Game/blueprint/instance/GameInstances Object Reference"))
  (bind _asgame_instances (cast `/Game/blueprint/instance/GameInstances` (`GameplayStatics.GetGameInstance` null)))
  (return _asgame_instances))

(fn `Get玩家`
  (returns (`AsBP Player` :type "/Game/blueprint/BP_player Object Reference"))
  (bind _asbp_player (cast `/Game/blueprint/BP_player` (`GameplayStatics.GetPlayerPawn` null)))
  (return _asbp_player))

(fn `检查是否在玩家范围内`
  (params (WorldLocation :type "Vector Structure"))
  (returns (ReturnValue :type Boolean))
  (bind (_x _y) (`KismetMathLibrary.BreakVector2D` (`WidgetLayoutLibrary.GetViewportSize` null)))
  (bind (_x_2 _y_2) (`KismetMathLibrary.BreakVector2D` (`PlayerController.ProjectWorldLocationToScreen` (`GameplayStatics.GetPlayerController` null) WorldLocation false)))
  (return (and (> _x_2 0.0) (> _y_2 0.0) (< _x_2 _x) (< _y_2 _y))))