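; Player character for a survivors-style game with 2D movement, item pickup, XP leveling, HP with brief post-hit invulnerability, and a game-over screen.
; Base stats load from a data asset and skills from SkillTable; level-ups open skill selection, and learned skills grant passive boosts or upgrade active ones.
; Active skills auto-fire on looping timers through the GameInstance's bullet pool: cursor-aimed darts and randomly placed lightning strikes around the player.
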(event `self.ReceiveBeginPlay`
  (bind `_as游戏实例` (`/Game/blueprint/instance/PublicLibraries.Get游戏实例`))
  ;[1 1 1] 初始化
  (`GameplayStatics.PlaySound2D` "/Game/sound/17_-_Fight.17_-_Fight" 1.0 1.0 0.0 null null)
  (set `/Game/blueprint/instance/GameInstances.玩家` self `_as游戏实例`)
  (set `self.As游戏实例` `_as游戏实例`)
  (`self.玩家数据初始化`)
  (`self.HUD初始化`)
  (bind _returnvalue (`|GetDataTableRow` "/Game/Data_assets/Skill_data/SkillTable.SkillTable" (`KismetStringLibrary.Conv_StringToName` (`self.初始技能`)))
    (:`then`
      (bind `_技能tag` (break `/Game/Data_assets/Skill_data/SkillStructure` _returnvalue))
      (`self.主动技能升级` `_技能tag`)
      (`self.自动释放主动技能` `_技能tag`))))

(event `EnhancedInput|/Game/Enhanced_inputs/IA_Move`
  (params (ActionValue :type "Vector2D Structure") (ElapsedSeconds :type "Float (double-precision)") (TriggeredSeconds :type "Float (double-precision)") (InputAction :type "InputAction Object Reference" :default "/Game/Enhanced_inputs/IA_Move.IA_Move"))
  (bind (_x _y) (`KismetMathLibrary.BreakVector2D` ActionValue))
  ;[1 1 1] 移动输入
  (:`Triggered`
    (set `self.X` _x)
    (set `self.Y` _y)
    (`self.AddMovementInput` (1.0 0.0 0.0) (`self.X`))
    (`self.AddMovementInput` (0.0 1.0 0.0) (`self.Y`))))

(event `/Game/interface/PlayerInterface.接收道具`
  (params (`道具` :type "/Game/道具/BP_Prop Object Reference"))
  ;[1 1 1] 接收道具
  (set `self.拾取的道具` `道具`)
  (switch `/Game/blueprint/enumerate/ItemClassification` (`/Game/道具/BP_Prop.道具分类` `道具`)
    (:`NewEnumerator1`
      (`self.增加经验值` (`/Game/道具/BP_Prop.经验值` (`self.拾取的道具`)))
      (`/Engine/EditorBlueprintResources/StandardMacros.IncrementInt` (`self.拾取金币数`)))
    (:`NewEnumerator2`
      (`SphereComponent.SetSphereRadius` (`self.道具拾取范围`) (`self.章鱼拾取范围`) true)
      (`KismetSystemLibrary.Delay` 3.0)
      (`SphereComponent.SetSphereRadius` (`self.道具拾取范围`) (`self.拾取范围`) true))))

(event `/Game/interface/PlayerInterface.玩家受击`
  (params (`伤害` :type "Float (double-precision)") (`攻击者` :type "Actor Object Reference"))
  ;[1 1 1] 玩家受击
  (`self.玩家受击HP变化` `伤害`))

(event `受击闪光`
  ;[1 1 1] 玩家受击
  (`GameplayStatics.PlaySound2D` "/Game/sound/sound_effect/PlayerHit.PlayerHit" 1.0 1.0 0.0 null null)
  (`PaperFlipbookComponent.SetSpriteColor` (`self.Sprite`) (struct :`R` 1.0 :`G` 0.0625 :`B` 0.0625 :`A` 1.0))
  (`KismetSystemLibrary.Delay` 0.2)
  (`PaperFlipbookComponent.SetSpriteColor` (`self.Sprite`) (struct :`R` 1.0 :`G` 1.0 :`B` 1.0 :`A` 1.0)))

(fn `HUD初始化`
  (bind _returnvalue (`|CreateWidget` "/Game/UI/UI_State.UI_State_C"))
  (bind _output_get (set `self.UI状态` _returnvalue))
  (`UserWidget.AddToViewport` _output_get 0)
  (`self.更新EXP界面`)
  (`self.更新HP界面`)
  (`self.更新击杀数`))

(fn `UserConstructionScript`)

(fn `主动技能升级`
  (params (`技能Tag` :type "String (by ref)"))
  (switch `string` `技能Tag`
    (:`飞镖`
      (switch `int` (`BlueprintMapLibrary.Map_Find` (`self.技能 TAG组`) "飞镖")
        (:`2`
          (set `self.飞镖子弹大小` (1.3 1.3 1.3)))
        (:`3`
          (set `self.生命周期` 2.0)
          (set `self.飞镖数量` 2))
        (:`4`
          (set `self.飞镖子弹大小` (1.5 1.5 1.5)))
        (:`5`
          (set `self.飞镖数量` 3))))
    (:`落雷`
      (if (== (`self.落雷增益`) 0.0)
        (bind _returnvalue (`|GetDataTableRow` "/Game/Data_assets/Skill_data/SkillTable.SkillTable" "落雷")
          (:`then`
            (bind (`_技能tag` `_名字` `_技能描述` `_等级` `_最大等级` `_释放频率` `_图标` `_增益`) (break `/Game/Data_assets/Skill_data/SkillStructure` _returnvalue))
            (set `self.落雷增益` `_增益`)
            (`self.自动释放主动技能` `_技能tag`))))
      (switch `int` (`BlueprintMapLibrary.Map_Find` (`self.技能 TAG组`) "落雷")
        (:`1`
          (set `self.落雷命中范围` (2.0 2.0 2.0)))
        (:`2`
          (set `self.落雷增益` (+ (`self.落雷增益`) 5.0)))
        (:`3`
          (set `self.落雷数量` 2))
        (:`4`
          (set `self.落雷命中范围` (2.5 2.5 2.5)))
        (:`5`
          (set `self.落雷数量` 3)
          (set `self.落雷增益` (+ (`self.落雷增益`) 5.0)))))))

(fn `受击保护`
  (`PrimitiveComponent.SetCollisionResponseToChannel` (`self.CapsuleComponent`) "ECC_Pawn" "ECR_Overlap"))

(fn `增加经验值`
  (params (`经验值` :type Integer))
  (locals (`溢出经验` :type Integer))
  (bind _output_get (set `self.当前经验` (+ (`self.当前经验`) `经验值`)))
  (if (>= _output_get (`self.升级经验`))
    (set `local.溢出经验` (- (`self.当前经验`) (`self.升级经验`)))
    (`/Engine/EditorBlueprintResources/StandardMacros.IncrementInt` (`self.等级`)
      (:`  `
        (`self.计算升级所需经验值`)
        (set `self.当前经验` 0)
        (`self.增加经验值` (`local.溢出经验`))
        (`/Game/UI/UI_State.显示技能选择界面` (`self.UI状态`))))
    (else
      (`self.更新EXP界面`))))

(fn `学习技能`
  (params (`技能标签` :type String))
  (bind `_技能标签` (`local.技能标签`))
  (bind (_value _returnvalue) (`BlueprintMapLibrary.Map_Find` (`self.技能 TAG组`) `技能标签`))
  (if _returnvalue
    (bind _result (`/Engine/EditorBlueprintResources/StandardMacros.IncrementInt` _value)
      (:`  `
        (`BlueprintMapLibrary.Map_Add` (`self.技能 TAG组`) (`local.技能标签`) _result)
        (for (_array_element _array_index) (`self.技能结构`)
          (bind (`_技能tag` `_名字` `_技能描述` `_等级` `_最大等级`) (break `/Game/Data_assets/Skill_data/SkillStructure` _array_element))
          (if (`KismetStringLibrary.EqualEqual_StrStr` `_技能tag` (`local.技能标签`))
            (if (== `_最大等级` _result)
              (`KismetArrayLibrary.Array_Remove` (`self.技能结构`) _array_index)
              (break))))))
    (else
      (`BlueprintMapLibrary.Map_Add` (`self.技能 TAG组`) (`local.技能标签`) 1)))
  (`/Game/UI/UI_State.刷新学到的技能` (`self.UI状态`))
  (`self.被动技能效果增益` `_技能标签`)
  (`self.主动技能升级` `_技能标签`))

(fn `更新EXP界面`
  (`/Game/UI/UI_State.更新exp` (`self.UI状态`) (`self.当前经验`) (`self.升级经验`))
  (`/Game/UI/UI_State.更新lv+exp` (`self.UI状态`) (`self.等级`) (`self.当前经验`) (`self.升级经验`)))

(fn `更新HP界面`
  (`/Game/UI/UI_State.更新HP` (`self.UI状态`) (`self.HP`) (`self.Hp Max`)))

(fn `更新击杀数`
  (`/Game/UI/UI_State.更新击杀数` (`self.UI状态`) (`self.击杀数`)))

(fn `玩家受击HP变化`
  (params (`伤害` :type "Float (double-precision)"))
  (set `self.HP` (`KismetMathLibrary.FClamp` (- (`self.HP`) `伤害`) 0.0 (`self.Hp Max`)))
  (`self.受击闪光`)
  (if (<= (`self.HP`) 0.0)
    (set `self.是否死亡` true)
    (`self.更新HP界面`)
    (`GameplayStatics.SetGamePaused` true)
    (bind _returnvalue (`|CreateWidget` "/Game/UI/UI_End.UI_End_C"))
    (bind _output_get (set `self.UI_End` _returnvalue))
    (`UserWidget.AddToViewport` _output_get 0)
    (else
      (`KismetSystemLibrary.K2_SetTimer` null "受击保护" 1.0)
      (`PrimitiveComponent.SetCollisionResponseToChannel` (`self.CapsuleComponent`) "ECC_Pawn" "ECR_Ignore")
      (`self.更新HP界面`))))

(fn `玩家数据初始化`
  (locals (NewLocalVar :type Integer :default 0))
  (bind (`_等级` _hpmax `_攻击力` `_移动速度` `_拾取范围` `_升级所需经验值` `_初始技能` `_升级基准值`) (`/Game/Data_assets/Player_data/Player_data.读取数据资产` (`self.玩家数据资产`)))
  (set `self.等级` `_等级`)
  (set `self.Hp Max` _hpmax)
  (set `self.攻击力` `_攻击力`)
  (set `self.移动速度` `_移动速度`)
  (set `self.拾取范围` `_拾取范围`)
  (set `self.初始技能` `_初始技能`)
  (set `CharacterMovementComponent.MaxWalkSpeed` (`self.移动速度`) (`self.CharacterMovement`))
  (`SphereComponent.SetSphereRadius` (`self.道具拾取范围`) (`self.拾取范围`) true)
  (set `self.HP` (`self.Hp Max`))
  (set `self.升级经验值基准` `_升级所需经验值`)
  (set `self.升级基准值` `_升级基准值`)
  (`BlueprintMapLibrary.Map_Add` (`self.技能 TAG组`) (`self.初始技能`) 1)
  (`self.计算升级所需经验值`)
  (bind _outrownames (`DataTableFunctionLibrary.GetDataTableRowNames` "/Game/Data_assets/Skill_data/SkillTable.SkillTable"))
  (for _array_element _outrownames
    (bind _returnvalue (`|GetDataTableRow` "/Game/Data_assets/Skill_data/SkillTable.SkillTable" _array_element)
      (:`then`
        (`KismetArrayLibrary.Array_Add` (`self.技能结构`) _returnvalue)))))

(fn `移除满级技能`
  (params (`技能结构` :type "/Game/Data_assets/Skill_data/SkillStructure Structure (by ref)"))
  (`KismetArrayLibrary.Array_RemoveItem` (`self.技能结构`) `技能结构`))

(fn `自动释放主动技能`
  (params (`技能Tag` :type String))
  (switch `string` `技能Tag`
    (:`飞镖`
      (`KismetSystemLibrary.K2_SetTimer` null "飞镖" 0.8 true))
    (:`落雷`
      (`KismetSystemLibrary.K2_SetTimer` null "落雷" 2.0 true))))

(fn `落雷`
  (bind _returnvalue (`KismetMathLibrary.RandomFloatInRange` -30.0 30.0))
  (bind (_returnvalue_x _returnvalue_y _returnvalue_z) (`KismetMathLibrary.BreakVector` (`self.K2_GetActorLocation`)))
  (for _ (range (`self.落雷数量`))
    (`/Game/blueprint/bullet/ObjectManagement.设置子弹池` (`/Game/blueprint/instance/GameInstances.对象管理` (`self.As游戏实例`)) (`KismetMathLibrary.MakeVector` (+ _returnvalue_x _returnvalue) (+ _returnvalue_y _returnvalue) _returnvalue_z) "/Game/bullet/Falling_thunder/落雷.落雷" (+ (`self.攻击力`) (`self.落雷增益`)) (0.0 0.0 0.0) (`self.落雷大小`) (`self.落雷命中范围`) "敌人" 0.5 10.0)))

(fn `被动技能效果增益`
  (params (`技能标签` :type String))
  (switch `string` `技能标签`
    (:`增加攻击`
      (set `self.攻击力` (+ (`self.攻击力`) 1.0)))
    (:`增加生命`
      (set `self.HP` (+ (`self.HP`) 10.0))
      (`self.更新HP界面`))
    (:`增加移速`
      (set `self.移动速度` (+ (`self.移动速度`) 5.0))
      (set `CharacterMovementComponent.MaxWalkSpeed` (`self.移动速度`) (`self.CharacterMovement`)))
    (:`增加拾取范围`
      (set `self.拾取范围` (+ (`self.拾取范围`) 5.0))
      (`SphereComponent.SetSphereRadius` (`self.道具拾取范围`) (`self.拾取范围`) true))))

(fn `计算升级所需经验值`
  (set `self.升级经验` (* (`self.升级经验值基准`) (`KismetMathLibrary.MultiplyMultiply_FloatFloat` (`self.升级基准值`) (`KismetMathLibrary.Conv_IntToDouble` (- (`self.等级`) 1))))))

(fn `飞镖`
  (bind _returnvalue (`self.K2_GetActorLocation`))
  (bind `_飞镖子弹大小` (`self.飞镖子弹大小`))
  (bind (_returnvalue_roll _returnvalue_pitch _returnvalue_yaw) (`KismetMathLibrary.BreakRotator` (`KismetMathLibrary.FindLookAtRotation` _returnvalue (`.Location` (`GameplayStatics.BreakHitResult` (`PlayerController.GetHitResultUnderCursorByChannel` (`GameplayStatics.GetPlayerController` 0) "TraceTypeQuery1" true))))))
  (for _index (range (`self.飞镖数量`))
    (bind _returnvalue_2 (select `int` _index :`0` -20.0 :`1` 20.0 :`2` 0.0))
    (`/Game/blueprint/bullet/ObjectManagement.设置子弹池` (`/Game/blueprint/instance/GameInstances.对象管理` (`self.As游戏实例`)) _returnvalue "/Game/bullet/dart/子弹_小飞镖.子弹_小飞镖" (`self.攻击力`) (* (`KismetMathLibrary.Conv_RotatorToVector` (`KismetMathLibrary.MakeRotator` 0.0 0.0 (+ _returnvalue_yaw (select `int` (`self.飞镖数量`) :`0` 0.0 :`1` 0.0 :`2` _returnvalue_2 :`3` _returnvalue_2)))) 100) `_飞镖子弹大小` `_飞镖子弹大小` "敌人" (`self.生命周期`) 10.0)))